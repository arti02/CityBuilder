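; Game mode Blueprint, by its name, that ends the game once the yellow, purple, red and white amounts all reach zero.
; Tick polls the four counters, then clears all widgets, shows a QuitMenu and quits after a delay.
; With no one-shot guard, the menu is removed and recreated every frame while the delay runs.
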(event `self.ReceiveTick`
  (params (DeltaSeconds :type "Float (single-precision)"))
  (if (and (and (and (== (`self.AmountYellow`) 0) (== (`self.AmountPurple`) 0)) (== (`self.AmountRed`) 0)) (== (`self.AmountWhite`) 0))
    (`WidgetLayoutLibrary.RemoveAllWidgets`)
    (bind _returnvalue (`|CreateWidget` "/Game/MyContent/UI/QuitMenu.QuitMenu_C"))
    (`UserWidget.AddToViewport` _returnvalue 0)
    (`KismetSystemLibrary.Delay` 10.0)
    (`KismetSystemLibrary.QuitGame` null "Quit")))

(fn `UserConstructionScript`)