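; Player controller for a grid-based house-building game, handling camera input and building placement.
; Forwards axis, zoom and right-mouse drag input to the bpCameraController pawn.
; In placement mode, a preview actor follows a cursor trace, snapped to the nearest GridManager cell.
; Left click spawns the building if placement is valid and stock remains, occupies the cell, and updates game-mode house counts and score, scaled by house and cell type.
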(event `self.ReceiveBeginPlay`
  (`self.SetPlacementModeEnabled` true))

(event `InputAxis|CameraOrbit`
  (params (AxisValue :type "Float (single-precision)"))
  (bind _asbp_camera_controller (cast `/Game/MyContent/Blueprints/bpCameraController` (`self.K2_GetPawn`)))
  (`/Game/MyContent/Blueprints/bpCameraController.CameraOrbit` _asbp_camera_controller AxisValue))

(event `PlacementInfoUpdated`
  (params (InPlaceableActorType :type "/Game/MyContent/GameObjects/Objects/bpPlaceableAsset Class Reference") (InPlaceableMode :type "/Game/MyContent/GameObjects/Grid/BuildingTypeEnum Enum" :default "NewEnumerator3"))
  (bind _placeableactor (`self.PlaceableActor`))
  (set `self.PlaceableActorType` InPlaceableActorType)
  (bind _output_get (set `self.PlaceableBuildingType` InPlaceableMode))
  (if (`|EnumEquality` _output_get "NewEnumerator3")
    (`self.SetPlacementModeEnabled` false)
    (else
      (`/Engine/EditorBlueprintResources/StandardMacros.IsValid` _placeableactor
        (:`Is Valid`
          (`self.K2_DestroyActor` _placeableactor))
        (:`Is Not Valid`
          _))
      (`self.RefreshPlaceableBui;ding`))))

(event `InputAxis|Move Forward/Backward`
  (params (AxisValue :type "Float (single-precision)"))
  (bind _asbp_camera_controller (cast `/Game/MyContent/Blueprints/bpCameraController` (`self.K2_GetPawn`)))
  (`/Game/MyContent/Blueprints/bpCameraController.MoveForward` _asbp_camera_controller AxisValue))

(event `InputAxis|StrafeLeft/Rigth`
  (params (AxisValue :type "Float (single-precision)"))
  (bind _asbp_camera_controller (cast `/Game/MyContent/Blueprints/bpCameraController` (`self.K2_GetPawn`)))
  (`/Game/MyContent/Blueprints/bpCameraController.LeftRigthStrafe` _asbp_camera_controller AxisValue))

(event `InputAction|CameraZoomIn`
  (params (Key :type "Key Structure"))
  (:`Pressed`
    (bind _asbp_camera_controller (cast `/Game/MyContent/Blueprints/bpCameraController` (`self.K2_GetPawn`)))
    (`/Game/MyContent/Blueprints/bpCameraController.CameraZoom` _asbp_camera_controller -1.0)))

(event `InputAction|CameraZoomOut`
  (params (Key :type "Key Structure"))
  (:`Pressed`
    (bind _asbp_camera_controller (cast `/Game/MyContent/Blueprints/bpCameraController` (`self.K2_GetPawn`)))
    (`/Game/MyContent/Blueprints/bpCameraController.CameraZoom` _asbp_camera_controller 1.0)))

(event `InputAxis|CameraPitch`
  (params (AxisValue :type "Float (single-precision)"))
  (bind _asbp_camera_controller (cast `/Game/MyContent/Blueprints/bpCameraController` (`self.K2_GetPawn`)))
  (`/Game/MyContent/Blueprints/bpCameraController.CameraPitch` _asbp_camera_controller AxisValue))

(event `InputAction|MouseRigthClick`
  (params (Key :type "Key Structure"))
  (:`Pressed`
    (set `self.RigthButtonPressed` true))
  (:`Released`
    (set `self.RigthButtonPressed` false)))

(event `InputAxis|Mouse X`
  (params (AxisValue :type "Float (single-precision)"))
  (if (`self.RigthButtonPressed`)
    (bind _asbp_camera_controller (cast `/Game/MyContent/Blueprints/bpCameraController` (`self.K2_GetPawn`)))
    (`/Game/MyContent/Blueprints/bpCameraController.CameraOrbit` _asbp_camera_controller AxisValue)))

(event `InputAxis|Mouse Y`
  (params (AxisValue :type "Float (single-precision)"))
  (if (`self.RigthButtonPressed`)
    (bind _asbp_camera_controller (cast `/Game/MyContent/Blueprints/bpCameraController` (`self.K2_GetPawn`)))
    (`/Game/MyContent/Blueprints/bpCameraController.CameraPitch` _asbp_camera_controller AxisValue)))

(event `self.ReceiveTick`
  (params (DeltaSeconds :type "Float (single-precision)"))
  (if (`self.PlacementModeEnabled`)
    (`self.UpdatePlacement`)))

(event `InputAction|MouseLeftClick`
  (params (Key :type "Key Structure"))
  (:`Pressed`
    (if (`self.PlacementModeEnabled`)
      (`self.SpawnBuilding`))))

(fn `ChangeAmountOfHouses`
  (params (`Placeable Object` :type "/Game/MyContent/GameObjects/Objects/bpPlaceableAsset Object Reference"))
  (bind _returnvalue (`GameplayStatics.GetGameMode`))
  (if (== (`GameplayStatics.GetObjectClass` `Placeable Object`) "/Game/MyContent/GameObjects/Objects/PurpleHouse.PurpleHouse_C")
    (bind _asbp_my_game_mod (cast `/Game/MyContent/Blueprints/bpMyGameMod` (`GameplayStatics.GetGameMode`)))
    (set `/Game/MyContent/Blueprints/bpMyGameMod.AmountPurple` (- (`/Game/MyContent/Blueprints/bpMyGameMod.AmountPurple` _asbp_my_game_mod) 1) _asbp_my_game_mod)
    (elif (== (`GameplayStatics.GetObjectClass` `Placeable Object`) "/Game/MyContent/GameObjects/Objects/YellowHouse.YellowHouse_C")
      (bind _asbp_my_game_mod_2 (cast `/Game/MyContent/Blueprints/bpMyGameMod` _returnvalue))
      (set `/Game/MyContent/Blueprints/bpMyGameMod.AmountYellow` (- (`/Game/MyContent/Blueprints/bpMyGameMod.AmountYellow` _asbp_my_game_mod_2) 1) _asbp_my_game_mod_2)
      (elif (== (`GameplayStatics.GetObjectClass` `Placeable Object`) "/Game/MyContent/GameObjects/Objects/WhiteHouse.WhiteHouse_C")
        (bind _asbp_my_game_mod_3 (cast `/Game/MyContent/Blueprints/bpMyGameMod` _returnvalue))
        (set `/Game/MyContent/Blueprints/bpMyGameMod.AmountWhite` (- (`/Game/MyContent/Blueprints/bpMyGameMod.AmountWhite` _asbp_my_game_mod_3) 1) _asbp_my_game_mod_3)
        (elif (== (`GameplayStatics.GetObjectClass` `Placeable Object`) "/Game/MyContent/GameObjects/Objects/RedHouse.RedHouse_C")
          (bind _asbp_my_game_mod_4 (cast `/Game/MyContent/Blueprints/bpMyGameMod` _returnvalue))
          (set `/Game/MyContent/Blueprints/bpMyGameMod.AmountRed` (- (`/Game/MyContent/Blueprints/bpMyGameMod.AmountRed` _asbp_my_game_mod_4) 1) _asbp_my_game_mod_4))))))

(fn `MultDivideScoreFromGrid`
  (params (House :type "/Game/MyContent/GameObjects/Objects/bpPlaceableAsset Object Reference") (GreedColor :type "/Game/MyContent/GameObjects/Grid/GridCellParent Object Reference"))
  (returns (ReturnScore :type Integer))
  (bind _returnvalue (`GameplayStatics.GetObjectClass` House))
  (bind _returnvalue_2 (`GameplayStatics.GetObjectClass` House))
  (bind _points_per_house (`/Game/MyContent/GameObjects/Objects/bpPlaceableAsset.Points Per House` House))
  (bind _returnvalue_3 (/ _points_per_house 2))
  ;[1 1 1] Green Grid
  (if (== (`GameplayStatics.GetObjectClass` GreedColor) "/Game/MyContent/GameObjects/Grid/GreenGridCell.GreenGridCell_C")
    (if (== _returnvalue_2 "/Game/MyContent/GameObjects/Objects/WhiteHouse.WhiteHouse_C")
      (`KismetSystemLibrary.PrintString` "You score multiply by 2")
      (return (* _points_per_house 2))
      (elif (== _returnvalue_2 "/Game/MyContent/GameObjects/Objects/YellowHouse.YellowHouse_C")
        (return (* _points_per_house 2))
        (else
          (return _points_per_house))))
    (else
      ;[1 1 1] Gray Greed
      (if (== (`GameplayStatics.GetObjectClass` GreedColor) "/Game/MyContent/GameObjects/Grid/GrayGreedCell.GrayGreedCell_C")
        _
        (else
          _))
      (if (== _returnvalue "/Game/MyContent/GameObjects/Objects/PurpleHouse.PurpleHouse_C")
        (return (* _points_per_house 2))
        (elif (== _returnvalue "/Game/MyContent/GameObjects/Objects/WhiteHouse.WhiteHouse_C")
          (return _returnvalue_3)
          (elif (== _returnvalue "/Game/MyContent/GameObjects/Objects/RedHouse.RedHouse_C")
            (return _returnvalue_3)
            (else
              (return _points_per_house))))))))

(fn `RefreshPlaceableBui;ding`
  (bind _returnvalue (`|SpawnActorFromClass` (`self.PlaceableActorType`) (`KismetMathLibrary.MakeTransform` (0.0 0.0 -100000.0)) "AlwaysSpawn" "OverrideRootScale" null null))
  (bind _asbp_placeable_asset (cast `/Game/MyContent/GameObjects/Objects/bpPlaceableAsset` _returnvalue)
    (:`then`
      (bind _output_get (set `self.PlaceableActor` _asbp_placeable_asset))
      (bind _returnvalue_2 (`self.GetComponentByClass` _output_get "/Game/MyContent/GameObjects/Components/bpClikableComponent.bpClikableComponent_C"))
      (`/Engine/EditorBlueprintResources/StandardMacros.IsValid` _returnvalue_2
        (:`Is Valid`
          (`/Game/MyContent/GameObjects/Components/bpClikableComponent.InplacementMode` _returnvalue_2))
        (:`Is Not Valid`
          _))
      (`AddComponent|NODE_AddbpPlopabbleComponent-0` :`self` _output_get))
    (:`CastFailed`
      (`AutomationBlueprintFunctionLibrary.AddExpectedLogError` "Actor of not pleaceable placcing type"))))

(fn `SetPlacementModeEnabled`
  (params (`Is Enabled` :type Boolean))
  (bind _placeableactor (`self.PlaceableActor`))
  (if (== `Is Enabled` (`self.PlacementModeEnabled`))
    (return)
    (else
      (bind _output_get (set `self.PlacementModeEnabled` `Is Enabled`))
      (if _output_get
        (`self.RefreshPlaceableBui;ding`)
        (else
          (`/Engine/EditorBlueprintResources/StandardMacros.IsValid` _placeableactor
            (:`Is Valid`
              (`self.K2_DestroyActor` _placeableactor))))))))

(fn `SpawnBuilding`
  (bind _placeableactor (`self.PlaceableActor`))
  (bind _returnvalue (`self.GetComponentByClass` (`self.PlaceableActor`) "/Game/MyContent/GameObjects/Components/bpPlopabbleComponent.bpPlopabbleComponent_C"))
  (bind _amountofthistype (`/Game/MyContent/GameObjects/Objects/bpPlaceableAsset.AmountOfThisType` _placeableactor))
  (`/Engine/EditorBlueprintResources/StandardMacros.IsValid` _returnvalue
    (:`Is Valid`
      (if (`/Game/MyContent/GameObjects/Components/bpPlopabbleComponent.IsPlasementValid` _returnvalue)
        (if (> _amountofthistype 0)
          (bind _returnvalue_2 (`|SpawnActorFromClass` (`self.PlaceableActorType`) (`self.GetTransform` _placeableactor) "AlwaysSpawn" "OverrideRootScale" null null))
          (set `/Game/MyContent/GameObjects/Objects/bpPlaceableAsset.AmountOfThisType` (- _amountofthistype 1) _placeableactor)
          (bind _returnvalue_3 (`GameplayStatics.GetActorOfClass` "/Game/MyContent/GameObjects/Grid/GridManager.GridManager_C"))
          (bind _outputvector (`/Game/MyContent/GameObjects/Grid/GridManager.GetClosestGridCell` _returnvalue_3 (`self.K2_GetActorLocation` _placeableactor)))
          (bind _asbp_placeable_asset (cast `/Game/MyContent/GameObjects/Objects/bpPlaceableAsset` _returnvalue_2))
          (set `/Game/MyContent/GameObjects/Objects/bpPlaceableAsset.GridCelRef` _outputvector _asbp_placeable_asset)
          (`/Game/MyContent/GameObjects/Grid/GridCellParent.SetOccupied` _outputvector (`/Game/MyContent/GameObjects/Objects/bpPlaceableAsset.BuildingType` _asbp_placeable_asset) _returnvalue_2)
          (bind _asbp_my_game_mod (cast `/Game/MyContent/Blueprints/bpMyGameMod` (`GameplayStatics.GetGameMode`)))
          (set `/Game/MyContent/Blueprints/bpMyGameMod.AmountOfAllBuildings` (+ (`/Game/MyContent/Blueprints/bpMyGameMod.AmountOfAllBuildings` _asbp_my_game_mod) 1) _asbp_my_game_mod)
          (bind _returnscore (`self.MultDivideScoreFromGrid` _asbp_placeable_asset _outputvector))
          (set `/Game/MyContent/Blueprints/bpMyGameMod.Score` (+ _returnscore (`/Game/MyContent/Blueprints/bpMyGameMod.Score` _asbp_my_game_mod)) _asbp_my_game_mod)
          (`self.ChangeAmountOfHouses` _asbp_placeable_asset))))))

(fn `UpdatePlacement`
  (bind (_worldlocation _worlddirection) (`self.DeprojectMousePositionToWorld`))
  (bind _outhit (`KismetSystemLibrary.LineTraceSingle` _worldlocation (+ _worldlocation (* _worlddirection 10000.0)) "TraceTypeQuery3"))
  (bind (_bblockinghit _binitialoverlap _time _distance _location) (`GameplayStatics.BreakHitResult` _outhit))
  (if _bblockinghit
    (bind _returnvalue (`GameplayStatics.GetActorOfClass` "/Game/MyContent/GameObjects/Grid/GridManager.GridManager_C"))
    (bind _outputvector (`/Game/MyContent/GameObjects/Grid/GridManager.GetClosestGridPosition` _returnvalue _location))
    (`self.K2_SetActorLocation` (`self.PlaceableActor`) _outputvector false false)))

(fn `UserConstructionScript`)